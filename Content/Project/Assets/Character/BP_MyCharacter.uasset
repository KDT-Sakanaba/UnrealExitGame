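; Player character with Enhanced Input movement, lever interaction, health, and death handling.
; BeginPlay creates the HUD and loads key states from a DataTable into a local array and, if empty, the GameInstance.
; Capsule overlaps track the current actor and toggle door messages from GameInstance key and door status.
; Damage, also triggered by right mouse, broadcasts HP; at zero the mesh ragdolls with a death message, and the player restarts upon destruction.
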(event OnComponentEndOverlap(CapsuleComponent)
  (params (OverlappedComponent :type Primitive%20Component%20Object%20Reference) (OtherActor :type Actor%20Object%20Reference) (OtherComp :type Primitive%20Component%20Object%20Reference) (OtherBodyIndex :type Integer))
  (Variables|Default|SetOverlapActor 0)
  (Utilities|Casting|CastToBP_Door OtherActor)
  (Default|SetDisplayMessage (Variables|Default|GetUI) false "    "))

(event OnComponentBeginOverlap(CapsuleComponent)
  (params (OverlappedComponent :type Primitive%20Component%20Object%20Reference) (OtherActor :type Actor%20Object%20Reference) (OtherComp :type Primitive%20Component%20Object%20Reference) (OtherBodyIndex :type Integer) (bFromSweep :type Boolean) (SweepResult :type Hit%20Result%20Structure%20%28by%20ref%29))
  (bind _mygameinstance (Variables|Default|GetMyGameInstance))
  (bind _output_get (Variables|Default|SetOverlapActor OtherActor))
  (bind _asbp_door (Utilities|Casting|CastToBP_Door _output_get))
  (if (== (Variables|/Game/Project/Assets/BluePrint/Door/BP_Door.BP_Door_C|GetKeyName _asbp_door) "")
    (if (Variables|/Game/Project/Assets/BluePrint/Door/BP_Door.BP_Door_C|GetSwitchDoor _asbp_door)
      (Default|SetDisplayMessage (Variables|Default|GetUI) true))
    (else
      (switch Utilities|FlowControl|Switch|SwitchonEN_KeyStatus (Default|GetKeyStatus _mygameinstance (Variables|/Game/Project/Assets/BluePrint/Door/BP_Door.BP_Door_C|GetKeyName _asbp_door))
        (:NewEnumerator0
          (switch Utilities|FlowControl|Switch|SwitchonEN_DoorState (Default|GetDoorStatus _mygameinstance (Variables|/Game/Project/Assets/BluePrint/Door/BP_Door.BP_Door_C|GetKeyName _asbp_door))
            (:NewEnumerator1
              (Default|SetDisplayMessage (Variables|Default|GetUI) true))))
        (:NewEnumerator1
          (Default|SetDisplayMessage (Variables|Default|GetUI) false "     " :!label _label))
        (:NewEnumerator2
          (goto _label))))))

(event Input|EnhancedActionEvents|EnhancedInputActionIAMyAtion
  (params (ActionValue :type Boolean) (ElapsedSeconds :type Float%20%28double-precision%29) (TriggeredSeconds :type Float%20%28double-precision%29) (InputAction :type Input%20Action%20Object%20Reference :default "/Game/Project/Assets/Character/input/IAMyAtion.IAMyAtion"))
  (:Started
    (bind _overlapactor (Variables|Default|GetOverlapActor)
      (:then
        (bind _asbp_lever (Utilities|Casting|CastToBP_lever _overlapactor))
        (Default|ShiftLever _asbp_lever))
      (:else))))

(event Input|EnhancedActionEvents|EnhancedInputActionIAMyMove
  (params (ActionValue :type Vector%202D%20Structure) (ElapsedSeconds :type Float%20%28double-precision%29) (TriggeredSeconds :type Float%20%28double-precision%29) (InputAction :type Input%20Action%20Object%20Reference :default "/Game/Project/Assets/Character/input/IAMyMove.IAMyMove"))
  (bind _returnvalue (Pawn|GetControlRotation :!class /Script/Engine.Pawn))
  (Utilities|FlowControl|Sequence
    (:then_0
      (Pawn|Input|AddMovementInput (Math|Vector|GetRightVector (Math|Rotator|MakeRotator (.roll _returnvalue) 0.0 (.yaw _returnvalue))) (.x ActionValue) false))
    (:then_1
      (Pawn|Input|AddMovementInput (Math|Vector|GetForwardVector (Math|Rotator|MakeRotator 0.0 0.0 (.yaw (Pawn|GetControlRotation :!class /Script/Engine.Pawn)))) (.y ActionValue) false))))

(event Input|EnhancedActionEvents|EnhancedInputActionIAMyLook
  (params (ActionValue :type Vector%202D%20Structure) (ElapsedSeconds :type Float%20%28double-precision%29) (TriggeredSeconds :type Float%20%28double-precision%29) (InputAction :type Input%20Action%20Object%20Reference :default "/Game/Project/Assets/Character/input/IAMyLook.IAMyLook"))
  (Pawn|Input|AddControllerYawInput (.x ActionValue))
  (Pawn|Input|AddControllerPitchInput (.y ActionValue)))

(event Input|EnhancedActionEvents|EnhancedInputActionIAMyJump
  (params (ActionValue :type Boolean) (ElapsedSeconds :type Float%20%28double-precision%29) (TriggeredSeconds :type Float%20%28double-precision%29) (InputAction :type Input%20Action%20Object%20Reference :default "/Game/Project/Assets/Character/input/IAMyJump.IAMyJump"))
  (:Started
    (Character|Jump))
  (:Canceled
    (Character|StopJumping)))

(event EventBeginPlay
  (Utilities|FlowControl|Sequence
    (:then_0
      (bind _asbp_my_game_instance (Utilities|Casting|CastToBP_MyGameInstance (Game|GetGameInstance)))
      (Variables|Default|SetMyGameInstance _asbp_my_game_instance)
      (bind _returnvalue (UserInterface|CreateWidget "/Game/Project/Assets/BluePrint/Game_UI.Game_UI_C"))
      (bind _output_get (Variables|Default|SetUI _returnvalue))
      (UserInterface|Viewport|AddtoViewport _output_get 0)
      (CallFunction|InitializeKeyStatus)
      (bind _outrownames (DataTable|GetDataTableRowNames "/Game/Project/Assets/BluePrint/DT_KeyStatus.DT_KeyStatus"))
      (for _array_element _outrownames
        (bind _returnvalue_2 (Utilities|GetDataTableRow "/Game/Project/Assets/BluePrint/DT_KeyStatus.DT_KeyStatus" _array_element)
          (:then
            (Utilities|Array|Add (Variables|Default|GetKeyStatus) _returnvalue_2)))))
    (:then_1
      (bind _asプレイヤーコントローラー (Utilities|Casting|CastToPlayerController (Pawn|GetController)))
      (Input|AddMappingContext (PlayerController|LocalPlayerSubsystems|GetEnhancedInputLocalPlayerSubsystem _asプレイヤーコントローラー) "/Game/Project/Assets/Character/input/IMCMyCharacter.IMCMyCharacter" 0 "(bIgnoreAllPressedKeysUntilRelease=True,bForceImmediately=False,bNotifyUserSettings=False)"))))

(event EventDestroyed
  (Default|SetDisplayCenter (Variables|Default|GetUI) false)
  (Class|GameModeBase|RestartPlayer (Game|GetGameMode) (Game|GetPlayerController 0)))

(event EventTick
  (params (DeltaSeconds :type Float%20%28single-precision%29)))

(event Collision|EventActorBeginOverlap
  (params (OtherActor :type Actor%20Object%20Reference)))

(event EventControllerChanged
  (params (OldController :type Controller%20Object%20Reference) (NewController :type Controller%20Object%20Reference)))

(event Input|MouseEvents|RightMouseButton
  (params (Key :type Key%20Structure))
  (:Pressed
    (CallFunction|AnyDamage self 1e+01)))

(fn ConstructionScript
  (Variables|Default|SetCurentHP 1e+02))

(fn InitializeKeyStatus
  (if (Utilities|Map|IsEmpty (Variables|/Game/Project/Assets/BluePrint/BP_MyGameInstance.BP_MyGameInstance_C|GetKeyStatus (Variables|Default|GetMyGameInstance)))
    (bind _outrownames (DataTable|GetDataTableRowNames 0))
    (for _array_element _outrownames
      (bind _returnvalue (Utilities|GetDataTableRow "/Game/Project/Assets/BluePrint/DT_KeyStatus.DT_KeyStatus" _array_element)
        (:then
          (Default|SaveKeyEnstance (Variables|Default|GetMyGameInstance) (.KeyName (Utilities|Struct|BreakST_KeyStatus _returnvalue)) (.KeyStatus (Utilities|Struct|BreakST_KeyStatus _returnvalue))))))))

(fn UpdateKeyStatus
  (params (KeyName :type Name) (KeyStatus :type EN_KeyStatus%20Enum :default "EN_KeyStatus_MAX"))
  (LocalVariables|SetLocalKeyName KeyName)
  (LocalVariables|SetLocalKeyStatus KeyStatus)
  (for (_array_element _array_index) (Variables|Default|GetKeyStatus)
    (if (== (.KeyName (Utilities|Struct|BreakST_KeyStatus _array_element)) (LocalVariables|GetLocalKeyName))
      (Utilities|Array|SetArrayElem (Variables|Default|GetKeyStatus) _array_index (Utilities|Struct|MakeST_KeyStatus (LocalVariables|GetLocalKeyName) (LocalVariables|GetLocalKeyStatus))))))

(fn GetKeyStatus
  (params (KeyName :type Name))
  (LocalVariables|SetlocalKeyName KeyName)
  (for _array_element (Variables|Default|GetKeyStatus)
    (if (== (.KeyName (Utilities|Struct|BreakST_KeyStatus _array_element)) (LocalVariables|GetlocalKeyName))
      (return (.KeyStatus (Utilities|Struct|BreakST_KeyStatus _array_element)))))
  (return "NewEnumerator0"))

(fn DeadEvent
  (Input|DisableInput 0)
  (Collision|SetCollisionProfileName (Variables|Character|GetMesh) "Ragdoll" true :!class /Script/Engine.PrimitiveComponent)
  (Physics|SetSimulatePhysics (Variables|Character|GetMesh) true)
  (Default|SetDisplayCenter (Variables|Default|GetUI) true "あなた死亡")
  (Actor|SetLifeSpan 3.0))

(fn UpdateMessage
  (bind _overlapactor (Variables|Default|GetOverlapActor)
    (:then
      (Utilities|Casting|CastToBP_Door _overlapactor))
    (:else)))

(fn AnyDamage
  (params (Damage :type Float%20%28double-precision%29))
  (bind _output_get (Variables|Default|SetCurentHP (- (Variables|Default|GetCurentHP) Damage)))
  (Default|CallOnCharacterHpChange (Variables|Default|GetCurentHP) 1e+02)
  (if (<= _output_get 0.0)
    (CallFunction|DeadEvent)))