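; BP_Door is a door that opens when BP_MyCharacter enters its box trigger, either directly or using a key.
; If KeyName is set or SwitchDoor is on, it requires that key's Get status in MyGameInstance, which it resets to Defort.
; Opening saves the door status and plays a timeline rotating the mesh's yaw.
; SetEventFinish extends the parent's, snapping the door open and disabling trigger collision.
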(event OnComponentBeginOverlap(Box)
  (params (OverlappedComponent :type Primitive%20Component%20Object%20Reference) (OtherActor :type Actor%20Object%20Reference) (OtherComp :type Primitive%20Component%20Object%20Reference) (OtherBodyIndex :type Integer) (bFromSweep :type Boolean) (SweepResult :type Hit%20Result%20Structure%20%28by%20ref%29))
  (Utilities|Casting|CastToBP_MyCharacter OtherActor)
  (if (and (== (Variables|Default|GetKeyName) "") (not (Variables|Default|GetSwitchDoor)))
    _
    (else
      (switch Utilities|FlowControl|Switch|SwitchonEN_KeyStatus (Default|GetKeyStatus (Variables|Default|GetMyGameInstance) (Variables|Default|GetKeyName))
        (:NewEnumerator1
          (Default|SaveKeyEnstance (Variables|Default|GetMyGameInstance) (Variables|Default|GetKeyName) "NewEnumerator0")))))
  (CallFunction|OpenDoor))

(event Custom|OpenDoor
  (Variables|Default|SetSwitchDoor false)
  (Default|SaveDoorStatus (Variables|Default|GetMyGameInstance) (Variables|Default|GetDoorName) "NewEnumerator1")
  (bind _trackz (Timeline|タイムライン Play)
    (:Update
      (Transformation|SetRelativeRotation (Variables|Default|GetSTM_Door) (Math|Rotator|MakeRotator 0.0 0.0 _trackz) false false))))

(event EventBeginPlay
  (|CallParentFunction))

(event Collision|EventActorBeginOverlap
  (params (OtherActor :type Actor%20Object%20Reference)))

(event EventTick
  (params (DeltaSeconds :type Float%20%28single-precision%29)))

(fn ConstructionScript)

(fn SetEventFinish
  (|CallParentFunction)
  (Variables|Default|SetSwitchDoor false)
  (Transformation|SetRelativeRotation (Variables|Default|GetSTM_Door) "0.000000,90.000000,0.000000" false false)
  (Collision|SetCollisionEnabled (Variables|Default|GetBox) "NoCollision"))