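; Pressure button gimmick that triggers a linked door or moving floor when BP_MyCharacter overlaps its box.
; The SwitchON timeline animates the button mesh's Z position, then on finish opens DoorOpen and activates MoveFloor's root component, whichever are valid.
; Only the door path calls SetEventFinish, which runs the parent's version, sets the mesh's relative location to zero and disables box collision.
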(event OnComponentBeginOverlap(Box)
  (params (OverlappedComponent :type Primitive%20Component%20Object%20Reference) (OtherActor :type Actor%20Object%20Reference) (OtherComp :type Primitive%20Component%20Object%20Reference) (OtherBodyIndex :type Integer) (bFromSweep :type Boolean) (SweepResult :type Hit%20Result%20Structure%20%28by%20ref%29))
  (Utilities|Casting|CastToBP_MyCharacter OtherActor)
  (bind _posz (Timeline|SwitchON Play)
    (:Update
      (Transformation|SetRelativeLocation (Variables|Default|GetSTM_Button) (Math|Vector|MakeVector 0.0 0.0 _posz) false false))
    (:Finished
      (Utilities|FlowControl|Sequence
        (:then_0
          (bind _dooropen (Variables|Default|GetDoorOpen)
            (:then
              (Default|OpenDoor _dooropen)
              (CallFunction|SetEventFinish))
            (:else)))
        (:then_1
          (bind _movefloor (Variables|Default|GetMoveFloor)
            (:then
              (Components|Activation|SetActive (Variables|/Script/Engine.Actor|GetRootComponent _movefloor) true false))
            (:else)))))))

(event EventBeginPlay
  (|CallParentFunction))

(event Collision|EventActorBeginOverlap
  (params (OtherActor :type Actor%20Object%20Reference)))

(event EventTick
  (params (DeltaSeconds :type Float%20%28single-precision%29)))

(fn ConstructionScript)

(fn SetEventFinish
  (|CallParentFunction)
  (Transformation|SetRelativeLocation (Variables|Default|GetSTM_Button) "0, 0, 0" false false)
  (Collision|SetCollisionEnabled (Variables|Default|GetBox) "NoCollision"))