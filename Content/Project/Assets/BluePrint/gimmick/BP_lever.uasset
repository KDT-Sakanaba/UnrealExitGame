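; Lever gimmick actor that opens a linked door once pulled.
; The shiftlever event plays the MoveLever timeline, which drives the pitch of the STMLever component's relative rotation.
; When the timeline finishes, it calls OpenDoor on the DoorOpen reference and then SetEventFinish, both only if that reference is valid.
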(event Custom|shift%20lever
  (bind _新規track_0 (Timeline|MoveLever Play)
    (:Update
      (Transformation|SetRelativeRotation (Variables|Default|GetSTM_Lever) (Math|Rotator|MakeRotator 0.0 _新規track_0 0.0) false false))
    (:Finished
      (bind _dooropen (Variables|Default|GetDoorOpen)
        (:then
          (Default|OpenDoor _dooropen)
          (CallFunction|SetEventFinish))
        (:else)))))

(event EventBeginPlay
  (|CallParentFunction) ; このノードは無効になっているため呼び出せません。\n機能をビルドするにはピンをドラッグしてください。
)

(event Collision|EventActorBeginOverlap
  (params (OtherActor :type Actor%20Object%20Reference))
  (|CallParentFunction OtherActor) ; このノードは無効になっているため呼び出せません。\n機能をビルドするにはピンをドラッグしてください。
)

(event EventTick
  (params (DeltaSeconds :type Float%20%28single-precision%29))
  (|CallParentFunction DeltaSeconds) ; このノードは無効になっているため呼び出せません。\n機能をビルドするにはピンをドラッグしてください。
)

(fn ConstructionScript
  (|CallParentFunction))